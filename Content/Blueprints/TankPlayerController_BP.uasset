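; Player controller Blueprint for a tank that sets up the player's on-screen UI.
; A How To Play screen is added to the viewport on BeginPlay at zero opacity and becomes visible only while the HowToPlay input is held, by toggling render opacity.
; The FoundAimingComponent event creates the PlayerUI widget and passes it the aiming component reference before adding it to the viewport.
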(event EventFoundAimingComponent
  (params (_AimCompRef :type Tank%20Aiming%20Component%20Object%20Reference))
  (bind _returnvalue (UserInterface|CreateWidget "/Game/UI/PlayerUI.PlayerUI_C"))
  (Variables|/Game/UI/PlayerUI.PlayerUI_C|SetBP%20Aiming%20Comp%20Reference _returnvalue _AimCompRef)
  (UserInterface|Viewport|AddtoViewport _returnvalue 0))

(event EventBeginPlay
  (bind _returnvalue (UserInterface|CreateWidget "/Game/UI/HowToPlayScreen.HowToPlayScreen_C"))
  (Widget|SetRenderOpacity _returnvalue 0.0)
  (UserInterface|Viewport|AddtoViewport _returnvalue 0))

(event Input|ActionEvents|InputActionHowToPlay
  (params (Key :type Key%20Structure))
  (:Pressed
    (bind _output_get (Variables|Default|SetHowToPlay (stale EventBeginPlay _returnvalue)))
    (Widget|SetRenderOpacity _output_get 1.0))
  (:Released
    (bind _output_get_2 (Variables|Default|SetHowToPlay (stale EventBeginPlay _returnvalue)))
    (Widget|SetRenderOpacity _output_get_2 0.0)))

(fn ConstructionScript)